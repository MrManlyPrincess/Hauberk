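; QueuedMovesComponent is a component that stores a single queued move for its owner.
; It exposes functions to get, set and clear that move, and setting a new one replaces the current one.
; When ClearMoveIfAddingDuplicate is on, setting a move of the same type as the queued one clears the slot instead, acting as a toggle.
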(fn GetQueuedMove
  (return (Variables|Default|GetQueueMove)))

(fn SetQueuedMove
  (params (Move :type Queued%20Move%20Object%20Reference))
  (if (Variables|Default|GetClearMoveIfAddingDuplicate)
    (if (Utilities|Enum|Equal(Enum) (Default|GetMoveType Move) (Default|GetMoveType (Variables|Default|GetQueueMove)))
      (Variables|Default|SetQueueMove 0)
      (else
        (Variables|Default|SetQueueMove Move :!label _label)))
    (else
      (goto _label))))

(fn ClearQueuedMove
  (Variables|Default|SetQueueMove 0))