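; Debug HUD that prints the player combat character's live state as on-screen text.
; Each frame, DrawHUD casts the controlled pawn to CombatCharacter and draws nothing if the cast fails.
; It draws color-coded lines in the top-left for health, stamina, lock-on status, and combat and movement states.
; The lock-on target line appears only while locked on to a valid target.
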(event EventDrawHUD
  (params (SizeX :type Integer) (SizeY :type Integer))
  (bind _ascombat_character (Utilities|Casting|CastToCombatCharacter (Pawn|GetControlledPawn (Variables|Default|GetPlayerOwner))))
  (HUD|DrawText (Utilities|String|ToString(Text) (Utilities|Text|FormatText "Health: {0}" (Utilities|Text|ToText(Float) (Class|HealthComponent|GetHealth (Variables|/Script/Hauberk.BaseCharacter|GetPlayerHealth _ascombat_character)) "HalfToEven" true 1 324 0 0))) "(R=0.000000,G=1.000000,B=0.981520,A=1.000000)" 1e+01 1e+01 0 1.0 false)
  (HUD|DrawText (Utilities|String|ToString(Text) (Utilities|Text|FormatText "Stamina: {0}" (Utilities|Text|ToText(Float) (Class|StaminaComponent|GetStamina (Variables|/Script/Hauberk.BaseCharacter|GetPlayerStamina _ascombat_character)) "HalfToEven" true 1 324 0 0))) "(R=0.000000,G=1.000000,B=0.000000,A=1.000000)" 1e+01 3e+01 0 1.0 false)
  (HUD|DrawText (Utilities|String|ToString(Text) (Utilities|Text|FormatText "IsLockedOn: {0}" (Utilities|Text|ToText(Boolean) (Variables|/Script/Hauberk.BaseCharacter|GetbIsLockedOn _ascombat_character)))) "(R=1.000000,G=0.000000,B=0.000000,A=1.000000)" 1e+01 5e+01 0 1.0 false)
  (if (Variables|/Script/Hauberk.BaseCharacter|GetbIsLockedOn _ascombat_character)
    (Utilities|IsValid (Variables|/Script/Hauberk.BaseCharacter|GetTarget_LockOn _ascombat_character)
      (:Is%20Valid
        (HUD|DrawText (Utilities|String|ToString(Text) (Utilities|Text|FormatText "LockTarget: {0}" (Utilities|Text|ToText(Object) (Variables|/Script/Hauberk.BaseCharacter|GetTarget_LockOn _ascombat_character)))) "(R=0.370000,G=0.290002,B=0.000000,A=1.000000)" 1e+01 7e+01 0 1.0 false))
      (:Is%20Not%20Valid
        _)))
  (HUD|DrawText (Utilities|String|ToString(Text) (Utilities|Text|FormatText "Combat State: {0}" (Utilities|Text|ToText(String) (Utilities|String|EnumtoString (Default|GetCombatState _ascombat_character))))) "(R=0.000000,G=0.000000,B=0.000000,A=1.000000)" 1e+01 9e+01 0 1.0 false)
  (HUD|DrawText (Utilities|String|ToString(Text) (Utilities|Text|FormatText "Movement State: {0}" (Utilities|Text|ToText(String) (Utilities|String|EnumtoString (Default|GetMovementState _ascombat_character))))) "(R=0.000000,G=0.000000,B=0.000000,A=1.000000)" 1e+01 1.1e+02 0 1.0 false))

(fn ConstructionScript)